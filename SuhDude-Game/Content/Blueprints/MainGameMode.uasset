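; Main game mode that adds the overlay widget at start, keeps the running score and handles the end of a game.
; AffectScore adjusts the score, and EndOfGame copies it to the game instance as the last score.
; EndOfGame also creates or loads the HighScores save, stores the score when it beats the record through a comparison helper, and leads back to MenuLevel.
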(event `self.ReceiveBeginPlay`
  (bind _returnvalue (`|CreateWidget` "/Game/Menus/Overlaay.Overlaay_C"))
  (`UserWidget.AddToViewport` _returnvalue 0))

(event `/Game/Blueprints/interfaces/InteractableObject.AffectScore`
  (params (ScoreChange :type Integer))
  (set `self.Score` (+ (`self.Score`) ScoreChange)))

(event `EndOfGame`
  (bind _mysavegame (`self.MySaveGame`))
  (bind _asmy_game_instance (cast `/Game/MyGameInstance` (`GameplayStatics.GetGameInstance`)))
  ;[1 1 1] Saves The score if you get the newest highscore
  (set `/Game/MyGameInstance.LastScore` (`self.Score`) _asmy_game_instance)
  (bind _returnvalue (`GameplayStatics.DoesSaveGameExist` "HighScores"))
  (if _returnvalue
    (bind _returnvalue_2 (`GameplayStatics.LoadGameFromSlot` "HighScores"))
    (bind _asmy_save_game (cast `/Game/MySaveGame` _returnvalue_2))
    (set `self.MySaveGame` _asmy_save_game)
    (bind _returnvalue_3 (`self.IsHighScore>Score` _mysavegame)
      (:`then`
        (set `/Game/MySaveGame.HighScore` _returnvalue_3 _mysavegame)
        (`GameplayStatics.SaveGameToSlot` _mysavegame "HighScores" :!label _label))
      (:`else`
        _))
    (else
      (bind _returnvalue_4 (`GameplayStatics.CreateSaveGameObject` "/Game/MySaveGame.MySaveGame_C"))
      (bind _asmy_save_game_2 (cast `/Game/MySaveGame` _returnvalue_4))
      (set `self.MySaveGame` _asmy_save_game_2)
      (set `/Game/MySaveGame.HighScore` (`KismetMathLibrary.Conv_IntToDouble` (`self.Score`)) _asmy_save_game_2)
      (goto _label)))
  (`GameplayStatics.OpenLevel` "MenuLevel"))

(fn `UserConstructionScript`)