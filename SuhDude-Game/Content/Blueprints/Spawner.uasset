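; Score-driven spawner that, while ReadyToStart, adds score every tick and spawns actors at random points inside its box.
; A Delay on Tick paces spawns through CalculateDelay, whose curve-based formula is marked unused.
; WhatToSpawn uses score and difficulty to pick the first class in the array or a random later one.
; With Arduino input enabled, BeginPlay clears ReadyToStart and overrides SpawnRate.
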(event `self.ReceiveBeginPlay`
  (bind _asmy_game_instance (cast `/Game/MyGameInstance` (`GameplayStatics.GetGameInstance`)))
  (if (`/Game/MyGameInstance.IsUsingArduino` _asmy_game_instance)
    (set `self.Ready to Start` false)
    (set `self.SpawnRate` 2.0)))

(event `self.ReceiveTick`
  (params (DeltaSeconds :type "Float (single-precision)"))
  (bind _returnvalue (`GameplayStatics.GetGameMode`))
  (bind _box (`self.Box`))
  (if (`self.Ready to Start`)
    (message `/Game/Blueprints/interfaces/InteractableObject.AffectScore` _returnvalue (`self.ScorePerTick`))
    (bind _asmain_game_mode (cast `/Game/Blueprints/MainGameMode` _returnvalue))
    (bind _score (`/Game/Blueprints/MainGameMode.Score` _asmain_game_mode))
    ;[1 1 1] Handles Spawning
    (`KismetSystemLibrary.Delay` (`self.CalculateDelay` _score))
    (bind _returnvalue_2 (`self.WhatToSpawn` _score (`self.Difficulty`)))
    (switch `int` _returnvalue_2
      (:`0`
        (set `self.IndexNumSpawn` 0))
      (:`1`
        (set `self.IndexNumSpawn` (`KismetMathLibrary.RandomIntegerInRange` 1 4))))
    (`|SpawnActorFromClass` (`KismetArrayLibrary.Array_Get` (`self.ArrayOfPossibleSpawn`) (`self.IndexNumSpawn`)) (`KismetMathLibrary.MakeTransform` (`KismetMathLibrary.RandomPointInBoundingBox` (`SceneComponent.K2_GetComponentLocation` _box) (`BoxComponent.GetScaledBoxExtent` _box)) (struct)) "Undefined" "OverrideRootScale")))

(fn `UserConstructionScript`)