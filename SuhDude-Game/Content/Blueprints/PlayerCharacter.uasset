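; Player character for a surfing game, which moves sideways on a board and tracks a balance value.
; MoveRight and an ArduinoMovement event share movement logic that tilts the capsule, offsets the actor and swaps spray effects by direction.
; AffectBalance caps balance at its maximum and calls the game mode's EndOfGame when it runs out.
; BeginPlay applies board and character sprites selected in the game instance; Q opens the menu level.
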(event `Key|Q`
  (params (Key :type "Key Structure" :default "AnyKey"))
  (:`Pressed`
    (`GameplayStatics.OpenLevel` "MenuLevel")))

(event `InputAxis|MoveRight`
  (params (AxisValue :type "Float (single-precision)"))
  (bind _axisvalue (`self.AxisValue`))
  (bind _capsulecomponent (`self.CapsuleComponent`))
  (bind _returnvalue_x (`KismetMathLibrary.BreakVector` (`KismetMathLibrary.Conv_DoubleToVector` _axisvalue)))
  (bind _returnvalue (* (* _returnvalue_x 90.0) -1.0))
  (set `self.AxisValue` AxisValue)
  ;[1 1 1] Changing Animation
  (`SceneComponent.SetVisibility` (`self.SideSprayLeft`) false false :!label _label)
  (`SceneComponent.SetVisibility` (`self.SideSprayRight`) false false)
  (`SceneComponent.SetVisibility` (`self.Spray`) false false)
  (if (== _axisvalue 0.0)
    (`SceneComponent.SetVisibility` (`self.Spray`) true false)
    (`SceneComponent.K2_SetRelativeRotation` _capsulecomponent (`KismetMathLibrary.MakeRotator` 0.0) false false)
    (else
      (if (> _axisvalue 0.0)
        (`SceneComponent.K2_SetRelativeRotation` _capsulecomponent (`KismetMathLibrary.MakeRotator` 0.0 _returnvalue) false false)
        (`SceneComponent.SetVisibility` (`self.SideSprayLeft`) true false)
        (else
          (`SceneComponent.K2_SetRelativeRotation` _capsulecomponent (`KismetMathLibrary.MakeRotator` 0.0 _returnvalue) false false)
          (`SceneComponent.SetVisibility` (`self.SideSprayRight`) true false)))
      (`self.K2_AddActorWorldOffset` (`KismetMathLibrary.MakeVector` (* _returnvalue_x 10.0)))))
  (set `self.AxisValue` 0.0))

(event `ArduinoMovement`
  (params (`Axis Value` :type "Float (double-precision)"))
  (set `self.AxisValue` `Axis Value`)
  (goto _label))

(event `/Game/Blueprints/interfaces/InteractableObject.AffectBalance`
  (params (BalanceChange :type "Float (single-precision)"))
  (bind _balance (`self.Balance`))
  ;[1 1 1] Balance
  (bind _output_get (set `self.Balance` (+ _balance BalanceChange)))
  (`self.ClampBalance` _output_get
    (:`else`
      _)
    (:`then`
      _))
  (if (<= _balance 0.0)
    (bind _asmain_game_mode (cast `/Game/Blueprints/MainGameMode` (`GameplayStatics.GetGameMode`)))
    (`/Game/Blueprints/MainGameMode.EndOfGame` _asmain_game_mode)))

(event `self.ReceiveBeginPlay`
  ;[1 1 1] Player selection sprite change
  (bind _asmy_game_instance (cast `/Game/MyGameInstance` (`GameplayStatics.GetGameInstance`)))
  (bind _output_get (set `self.MyGameInstanceVar` _asmy_game_instance))
  (`PaperSpriteComponent.SetSprite` (`self.SurfBoard`) (`KismetArrayLibrary.Array_Get` (`self.SurfBoardArray`) (`/Game/MyGameInstance.BoardSelctionPersistant` _output_get)))
  (`PaperSpriteComponent.SetSprite` (`self.Character`) (`KismetArrayLibrary.Array_Get` (`self.PlayerSpriteArray`) (`/Game/MyGameInstance.PlayerSelectionPersistant` (`self.MyGameInstanceVar`)))))

(fn `UserConstructionScript`)